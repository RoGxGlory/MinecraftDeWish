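; BP_ChunkActor is a chunk actor that handles mining of its targeted block.
; StartBreak compares elapsed time to the break time for the given mining force, then breaks the block and resets the player character's break event message.
; GetBlockData looks up the targeted block's row in Block_DataTable.
; GetHitFace wraps GetHitFaceAtLocation to return the face at a hit location.
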(event `/Game/Interfaces/BPI_Destroyable.StartBreak`
  (params (MiningForce :type "Float (double-precision)") (Time :type "Float (double-precision)"))
  (if (>= Time (`self.GetTargetedBlockBreakTime` MiningForce))
    (`self.BreakTargetedBlock`)
    (message `/Game/Interfaces/BPI_Destroyable.ResetBreakEvent` (`GameplayStatics.GetPlayerCharacter` 0))))

(fn `GetBlockData`
  (returns (BlockData :type "/Game/Data/S_Block_Data Structure"))
  (bind _returnvalue (`|GetDataTableRow` "/Game/Data/Block_DataTable.Block_DataTable" (`self.GetTargetedBlockRowName`))
    (:`then`
      (return _returnvalue))))

(fn `GetHitFace`
  (params (`Hit Location` :type "Vector Structure"))
  (returns (FaceID :type Integer))
  (return (`self.GetHitFaceAtLocation` `Hit Location`)))

(fn `UserConstructionScript`)