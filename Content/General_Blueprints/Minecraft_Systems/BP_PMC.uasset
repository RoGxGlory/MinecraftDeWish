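; BP_PMC is a Minecraft-style voxel chunk actor, still unfinished, that generates block data on BeginPlay.
; GenerateChunk sizes a flat block array for a 16×16×16 chunk, computes 1D Perlin surface heights and writes flattened indices without supplying block values or using those heights.
; Data table block lookups with debug printing and procedural mesh section creation with collision exist but never run.
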(event `self.ReceiveBeginPlay`
  (`self.GenerateChunk`))

(fn `GenerateChunk`
  (locals (Vertices :type "Array of Vector Structure") (Triangles :type "Array of Integer") (UVs :type "Array of Vector2D Structure") (Normals :type "Array of Vector Structure") (VertexColors :type "Array of LinearColor Structure") (Frequency :type "Float (double-precision)" :default 0.05) (SurfaceHeight :type "Float (double-precision)" :default 0.0))
  (bind _s_chunkdata_blocks (break `/Game/Data/S_ChunkData` (`self.S_ChunkData`)))
  (`KismetArrayLibrary.Array_Resize` (`.Blocks_6_1BFF7E414C5D586E9071499E63C226D6` (break `/Game/Data/S_ChunkData` (`self.S_ChunkData`))) 4096)
  (for _index (range 16)
    (for _index_2 (range 16)
      (set `local.SurfaceHeight` (`KismetMathLibrary.MapRangeClamped` (`KismetMathLibrary.PerlinNoise1D` (* (+ _index (* _index_2 100)) (`local.Frequency`))) 4.0 12.0 4.0 12.0)))
    (for _index_3 (range 16)
      (`KismetArrayLibrary.Array_Set` _s_chunkdata_blocks (+ (+ _index (* _index_2 16)) (* _index_3 256))))))

(fn `UserConstructionScript`)