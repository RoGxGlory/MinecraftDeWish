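; Player-side component for Minecraft-style block mining and inspection, built on look-at line traces and the BPI_Destroyable interface.
; BeginPlay caches the player character, creates the HUD and starts a looping timer that traces for the targeted block to show or hide its info.
; StartMining runs its own trace and sends the current mining force to the hit block.
; The timed check also queries the hit face, printed only in debug mode.
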(event `StartMining`
  (bind (_startpoint _endpoint) (`self.FindLookAt`))
  (bind (_outhit _returnvalue) (`KismetSystemLibrary.LineTraceSingle` :`Start` _startpoint :`End` _endpoint :`TraceChannel` "TraceTypeQuery1" :`DrawTime` 2.0))
  (if _returnvalue
    (if (`self.bDebug?`)
      (bind (_bblockinghit _binitialoverlap _time _distance _location _impactpoint _normal _impactnormal _physmat _hitactor) (`GameplayStatics.BreakHitResult` _outhit))
      (`KismetSystemLibrary.PrintText` (`|FormatText` "Hit Location : {HL} \nHit Actor : {HA}" (`KismetTextLibrary.Conv_VectorToText` _location) _hitactor)))
    (if (`KismetSystemLibrary.DoesImplementInterface` _hitactor "/Game/Interfaces/BPI_Destroyable.BPI_Destroyable_C")
      (message `/Game/Interfaces/BPI_Destroyable.StartBreak` _hitactor (`self.Current_Mining_Force`)))))

(event `Setup References`
  ; First step where references are set up
  (set `self.Player_Char` (`GameplayStatics.GetPlayerCharacter` 0)))

(event `Prepare Widget`
  ; Second step where UI elements are prepared and added to the viewport
  (bind _returnvalue (`|CreateWidget` "/Game/General_Blueprints/UI/WB_HUD.WB_HUD_C" (`GameplayStatics.GetPlayerController` 0)))
  (bind _output_get (set `self.HUD` _returnvalue))
  (`UserWidget.AddToViewport` _output_get 0))

(event `Setup Timers Logic`
  ; Third step where inner logic is set up
  (bind _returnvalue (`KismetSystemLibrary.K2_SetTimerDelegate` (delegate `CallLT`) (`self.TimeBeforeNextLTCheck`) true))
  (set `self.LTRepeatTimer` _returnvalue))

(event `ProcessLTCheck`
  (bind (_startpoint _endpoint) (`self.FindLookAt`))
  (bind (_outhit _returnvalue) (`KismetSystemLibrary.LineTraceSingle` :`Start` _startpoint :`End` _endpoint :`TraceChannel` "TraceTypeQuery1" :`DrawTime` 2.0))
  (if _returnvalue
    (bind (_bblockinghit _binitialoverlap _time _distance _location _impactpoint _normal _impactnormal _physmat _hitactor) (`GameplayStatics.BreakHitResult` _outhit))
    (if (`KismetSystemLibrary.DoesImplementInterface` _hitactor "/Game/Interfaces/BPI_Destroyable.BPI_Destroyable_C")
      (bind _blockdata (message `/Game/Interfaces/BPI_Destroyable.GetBlockData` _hitactor))
      (`/Game/General_Blueprints/UI/WB_BlockInfo.ProcessBlock` (`/Game/General_Blueprints/UI/WB_HUD.WB_BlockInfo` (`self.HUD`)) _blockdata)
      (bind _faceid (message `/Game/Interfaces/BPI_BuildSystem.GetHitFace` _hitactor _impactpoint))
      (if (`self.bDebug?`)
        (`KismetSystemLibrary.PrintText` (`|FormatText` (select `int` _faceid :`0` "Hit face : Front" :`1` "Hit face : Back" :`2` "Hit face : Left" :`3` "Hit face : Right" :`4` "Hit face : Top" :`5` "Hit face : Bottom" :!type "Text"))))
      (else
        (`/Game/General_Blueprints/UI/WB_BlockInfo.HideInfo` (`/Game/General_Blueprints/UI/WB_HUD.WB_BlockInfo` (`self.HUD`)) :!label _label)))
    (else
      (goto _label))))

(event `CallLT`
  ; Third step where inner logic is set up
  (`self.ProcessLTCheck`))

(event `self.ReceiveBeginPlay`
  ; Main system setup
  (`self.Setup References`)
  (`self.Prepare Widget`)
  (`self.Setup Timers Logic`))